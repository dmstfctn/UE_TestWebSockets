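; BP_SingleCam is a scene-capture camera actor whose orientation is driven remotely over Socket.IO.
; Its construction script creates a render target for the SceneCapture2D and feeds it into a dynamic M_BasicCamera material as the camera view.
; On connection it binds a "control" event, mapping JSON x and y values to actor yaw and pitch.
; StartCapturing and StopCapturing toggle the capture component's tick and visibility.
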(event OnConnected(SocketIOClient)
  (params (SessionId :type String) (bIsReconnection :type Boolean))
  (Development|PrintString "WS On Connected ")
  (Class|SocketIOClientComponent|BindEventtoGenericEvent (Variables|Default|GetSocketIOClient) "control" "/"))

(event OnGenericEvent(SocketIOClient)
  (params (EventName :type String) (MessageJson :type SIO%20Json%20Value%20Object%20Reference))
  (if (== EventName "control")
    (bind _returnvalue (Class|SIOJsonValue|AsObject MessageJson))
    (Transformation|SetActorRotation (Math|Rotator|MakeRotator 0.0 (Math|Float|MapRangeClamped (Class|SIOJsonObject|GetNumberField _returnvalue "y") -1.0 1.0 -9e+01 9e+01) (Math|Float|MapRangeClamped (Class|SIOJsonObject|GetNumberField _returnvalue "x") -1.0 1.0 -1.8e+02 1.8e+02)))))

(event EventBeginPlay)

(event Collision|EventActorBeginOverlap
  (params (OtherActor :type Actor%20Object%20Reference)))

(event EventTick
  (params (DeltaSeconds :type Float%20%28single-precision%29)))

(fn ConstructionScript
  (bind _returnvalue (Rendering|CreateRenderTarget2D (Variables|Default|GetTextureResolutionWidth) (Variables|Default|GetTextureResolutionHeight) "RTF_RGBA8_SRGB"))
  (bind _output_get (Variables|Default|SetT_RenderTarget _returnvalue))
  (Variables|/Script/Engine.SceneCaptureComponent2D|SetTextureTarget (Variables|Default|GetSceneCapture2d) _output_get)
  (bind _returnvalue_2 (Rendering|Material|CreateDynamicMaterialInstance "/Game/TestWebSockets/materials/M_BasicCamera.M_BasicCamera" "None" "None" :!class /Script/Engine.KismetMaterialLibrary))
  (Rendering|Material|SetTextureParameterValue _returnvalue_2 "BaseColor" (Variables|Default|GetT_RenderTarget))
  (Variables|Default|SetMI_CameraView _returnvalue_2)
  (Transformation|SetRelativeLocation (Variables|Default|GetSceneCapture2d) "0, 0, 0" false false))

(fn StopCapturing
  (bind _scenecapture2d (Variables|Default|GetSceneCapture2d))
  (Components|Tick|SetComponentTickEnabled _scenecapture2d false)
  (Rendering|SetVisibility _scenecapture2d false false))

(fn StartCapturing
  (bind _scenecapture2d (Variables|Default|GetSceneCapture2d))
  (Components|Tick|SetComponentTickEnabled _scenecapture2d true)
  (Rendering|SetVisibility _scenecapture2d true false))