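; BP_SocketReceiver is an actor that moves in response to messages from a Socket.IO server, apparently as a WebSocket test.
; When its SocketIOClient component connects, it binds the "control" event on the root namespace.
; Each control message's JSON x and y fields are added to the root's relative location to set the actor's position, without sweeping, leaving Z unchanged.
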(event OnConnected(SocketIOClient)
  (params (SessionId :type String) (bIsReconnection :type Boolean))
  (Development|PrintString "WS On Connected ")
  (Class|SocketIOClientComponent|BindEventtoGenericEvent (Variables|Default|GetSocketIOClient) "control" "/"))

(event OnGenericEvent(SocketIOClient)
  (params (EventName :type String) (MessageJson :type SIO%20Json%20Value%20Object%20Reference))
  (if (== EventName "control")
    (bind _returnvalue (Class|SIOJsonValue|AsObject MessageJson))
    (Transformation|SetActorLocation (+ (.Location (Math|Transform|BreakTransform (Transformation|GetRelativeTransform (Variables|Default|GetDefaultSceneRoot)))) (Math|Vector|MakeVector (Class|SIOJsonObject|GetNumberField _returnvalue "x") (Class|SIOJsonObject|GetNumberField _returnvalue "y") 0.0)) false false)))

(event EventBeginPlay
  (Development|PrintString "BeginPlay"))

(event Collision|EventActorBeginOverlap
  (params (OtherActor :type Actor%20Object%20Reference)))

(event EventTick
  (params (DeltaSeconds :type Float%20%28single-precision%29)))

(fn ConstructionScript)

(fn OnReceiveSocketId
  (params (id :type SIO%20Json%20Value%20Object%20Reference))
  (Development|PrintString (Class|SIOJsonValue|AsString id)))