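; BP_Multiplayer builds a split-screen grid view from multiple scene-capture cameras, toggled with the M key.
; On BeginPlay it spawns a BP_SingleCam per grid cell, spreading their yaw evenly around 360 degrees.
; Each camera feeds a WBP_SingleScreen placed in the uniform grid of WBP_SplitScreen.
; Toggling starts or stops every capture and adds or removes the container from the viewport.
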(event EventBeginPlay
  (bind _gridcolumncount (Variables|Default|GetGridColumnCount))
  (bind _gridrowcount (Variables|Default|GetGridRowCount))
  (bind _screenresolution (Variables|Default|GetScreenResolution))
  (Utilities|FlowControl|Sequence
    (:then_0
      ;[0 0 0] Create the main grid container
      (bind _returnvalue (UserInterface|CreateWidget "/Game/blueprints/WBP_SplitScreen.WBP_SplitScreen_C"))
      (Variables|Default|SetSplitScreenContainer _returnvalue))
    (:then_1
      (Utilities|Array|Clear (Variables|Default|GetScreens))
      (Utilities|Array|Clear (Variables|Default|GetCameras))
      (Variables|Default|SetGridCurrentIndex 0)
      (Variables|Default|SetGridTotalCount (* _gridcolumncount _gridrowcount))
      (for _index (range 0 (- _gridcolumncount 1))
        (Variables|Default|SetGridCurrentColumn _index)
        (for _index_2 (range 0 (- _gridrowcount 1))
          (Variables|Default|SetGridCurrentRow _index_2)
          (Utilities|FlowControl|Sequence
            (:then_0
              (bind _returnvalue_2 (Game|SpawnActorfromClass "/Game/blueprints/BP_SingleCam.BP_SingleCam_C" (Math|Transform|MakeTransform "0.000000,0.000000,50.000000" (Math|Rotator|MakeRotator 0.0 0.0 (* (/ 3.6e+02 (Math|Conversions|ToFloat(Integer) (Variables|Default|GetGridTotalCount))) (Variables|Default|GetGridCurrentIndex)))) "AlwaysSpawn" 0 _screenresolution _screenresolution 0))
              (Utilities|Array|Add (Variables|Default|GetCameras) _returnvalue_2)
              (bind _returnvalue_3 (UserInterface|CreateWidget "/Game/blueprints/WBP_SingleScreen.WBP_SingleScreen_C" 0 _returnvalue_2 (Variables|Default|GetScreenSize)))
              (Utilities|Array|Add (Variables|Default|GetScreens) _returnvalue_3)
              (Class|UniformGridPanel|AddChildtoUniformGrid (Variables|/Game/blueprints/WBP_SplitScreen.WBP_SplitScreen_C|GetGridPanel (Variables|Default|GetSplitScreenContainer)) _returnvalue_3 (Variables|Default|GetGridCurrentRow) (Variables|Default|GetGridCurrentColumn)))
            (:then_1
              (Math|Integer|IncrementInt (Variables|Default|GetGridCurrentIndex)))))))
    (:then_2
      (if (Variables|Default|GetIsActive)
        (UserInterface|Viewport|AddtoViewport (Variables|Default|GetSplitScreenContainer) 0)))
    (:then_3
      (Input|EnableInput (Class|GameplayStatics|GetPlayerControllerfromID)))))

(event EventTick
  (params (DeltaSeconds :type Float%20%28single-precision%29)))

(event Input|KeyboardEvents|M
  (params (Key :type Key%20Structure :default "None"))
  (bind _cameras (Variables|Default|GetCameras))
  (:Pressed
    (if (Variables|Default|GetIsActive)
      (for _array_element _cameras
        (Default|StopCapturing _array_element))
      (Variables|Default|SetIsActive false)
      (Widget|RemovefromParent (Variables|Default|GetSplitScreenContainer))
      (else
        (for _array_element_2 _cameras
          (Default|StartCapturing _array_element_2))
        (Variables|Default|SetIsActive true)
        (UserInterface|Viewport|AddtoViewport (Variables|Default|GetSplitScreenContainer) 0)))))

(fn ConstructionScript)