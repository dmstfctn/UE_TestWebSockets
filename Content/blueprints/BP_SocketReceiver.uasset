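; BP_SocketReceiver is an actor moved remotely by messages from its SocketIOClient component.
; On connection it binds the "control" event, then adds each message's JSON x and y fields to the root component's relative location, leaving Z, rotation and scale unchanged.
; Each message is thus an offset, not an absolute position.
; OnReceiveSocketId only prints an ID and is not bound or called here.
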(event OnConnected(SocketIOClient)
  (params (SessionId :type String) (bIsReconnection :type Boolean))
  (Development|PrintString "WS On Connected ")
  (Class|SocketIOClientComponent|BindEventtoGenericEvent (Variables|Default|GetSocketIOClient) "control" "/"))

(event OnGenericEvent(SocketIOClient)
  (params (EventName :type String) (MessageJson :type SIO%20Json%20Value%20Object%20Reference))
  (bind _defaultsceneroot (Variables|Default|GetDefaultSceneRoot))
  (bind _returnvalue (Transformation|GetRelativeTransform _defaultsceneroot))
  (bind (_location _rotation _scale) (Math|Transform|BreakTransform _returnvalue))
  (if (== EventName "control")
    (bind _returnvalue_2 (Class|SIOJsonValue|AsObject MessageJson))
    (Transformation|SetRelativeTransform _defaultsceneroot (Math|Transform|MakeTransform (+ _location (Math|Vector|MakeVector (Class|SIOJsonObject|GetNumberField _returnvalue_2 "x") (Class|SIOJsonObject|GetNumberField _returnvalue_2 "y") 0.0)) _rotation _scale) false false)))

(event EventBeginPlay
  (Development|PrintString "BeginPlay"))

(event Collision|EventActorBeginOverlap
  (params (OtherActor :type Actor%20Object%20Reference)))

(event EventTick
  (params (DeltaSeconds :type Float%20%28single-precision%29)))

(fn ConstructionScript)

(fn OnReceiveSocketId
  (params (id :type SIO%20Json%20Value%20Object%20Reference))
  (Development|PrintString (Class|SIOJsonValue|AsString id)))